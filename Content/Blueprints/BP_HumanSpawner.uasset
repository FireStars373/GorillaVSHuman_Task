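; Spawner actor that populates the level with humans and shows their count on the HUD.
; BeginPlay creates the WB_Humans widget, which SpawnHumans passes to every spawned actor as its HUD reference.
; SpawnHumans, not triggered within this graph, places each human at a random reachable navigation point within a fixed radius of the spawner.
; It then sets the widget's count to the spawn count and adds it to the viewport.
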(event `self.ReceiveBeginPlay`
  (bind _returnvalue (`|CreateWidget` "/Game/Widgets/WB_Humans.WB_Humans_C"))
  (set `self.HumanWidgetRef` _returnvalue))

(event `self.ReceiveTick`
  (params (DeltaSeconds :type "Float (single-precision)")))

(event `SpawnHumans`
  (bind _humanwidgetref (`self.HumanWidgetRef`))
  ; Human Spawning
  (for _ (range 1 (+ (`self.HumanSpawnCount`) 1))
    (`|SpawnActorFromClass` "/Game/Blueprints/BP_Human.BP_Human_C" (`KismetMathLibrary.MakeTransform` (`NavigationSystemV1.K2_GetRandomReachablePointInRadius` (`self.K2_GetActorLocation`) 7000.0 null null)) "AdjustIfPossibleButAlwaysSpawn" "MultiplyWithRoot" null (`self.HumanWidgetRef`) null)
    (`/Engine/EditorBlueprintResources/StandardMacros.IncrementInt` (`self.Humans`)))
  ;; Updats HUD with how many humans left
  (set `/Game/Widgets/WB_Humans.humans` (`self.HumanSpawnCount`) _humanwidgetref)
  (`UserWidget.AddToViewport` _humanwidgetref 0))

(fn `UserConstructionScript`)