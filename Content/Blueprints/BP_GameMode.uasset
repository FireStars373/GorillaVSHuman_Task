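; Game mode that runs a four-round wave game pitting the player's gorilla against growing numbers of humans.
; StartRound sets the human count for the current round and passes it to the first BP_HumanSpawner found in the level.
; CheckHumanCount decrements the survivors and, at zero, RoundEnd fully heals the gorilla and starts the next round.
; Tick accumulates total play time until the final round ends.
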(event `self.ReceiveBeginPlay`
  (`self.StartRound`)
  (set `self.LevelTime` 0.0)
  (set `self.TimerOn` true))

(event `self.ReceiveTick`
  (params (DeltaSeconds :type "Float (single-precision)"))
  ; Time Counter
  (if (`self.TimerOn`)
    (set `self.LevelTime` (+ (`self.LevelTime`) DeltaSeconds))))

(event `StartRound`
  ; Check Round and set Human Spawn Count
  (`|ExecutionSequence`
    (:`then_0`
      (switch `int` (`self.CurrentRound`)
        (:`0`
          (set `self.HumansAlive` 10))
        (:`1`
          (set `self.HumansAlive` 25))
        (:`2`
          (set `self.HumansAlive` 50))
        (:`3`
          (set `self.HumansAlive` 100))))
    (:`then_1`
      ;; Sends Human Count to spawn this Round
      (bind _outactors (`GameplayStatics.GetAllActorsOfClass` "/Game/Blueprints/BP_HumanSpawner.BP_HumanSpawner_C"))
      (bind _output (`|GetArrayItem` _outactors))
      (set `/Game/Blueprints/BP_HumanSpawner.HumanSpawnCount` (`self.HumansAlive`) _output)
      (`/Game/Blueprints/BP_HumanSpawner.SpawnHumans` _output))))

(event `CheckHumanCount`
  ; Check how many Humans are left and if none Ends Round
  (bind _result (`/Engine/EditorBlueprintResources/StandardMacros.DecrementInt` (`self.HumansAlive`))
    (:`  `
      (bind _output_get (set `self.HumansAlive` _result))
      (if (<= _output_get 0)
        (`self.RoundEnd`)))))

(event `RoundEnd`
  ; On Round End Heal Gorilla to Full, Set Next Round and Start it
  (bind _asbp_gorilla (cast `/Game/Blueprints/BP_Gorilla` (`GameplayStatics.GetPlayerCharacter` 0)))
  (`/Game/Blueprints/BP_Gorilla.FullHealGorilla` _asbp_gorilla)
  (bind _result (`/Engine/EditorBlueprintResources/StandardMacros.IncrementInt` (`self.CurrentRound`))
    (:`  `
      (set `self.CurrentRound` _result)
      (set `self.HumansAlive` 0)
      (if (>= (`self.CurrentRound`) 4)
        (set `self.TimerOn` false)
        (else
          (`self.StartRound`))))))

(fn `UserConstructionScript`)