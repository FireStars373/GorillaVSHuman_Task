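; BP_Human is an enemy AI character that chases the player from BeginPlay or on sight and punches on reaching them.
; A hand sphere, switched by ToggleHumanCollision, applies damage when it overlaps the player.
; The first damage taken kills it: the mesh ragdolls with a backward impulse, pain sound and blood effect.
; Death decrements the HUD human count and has BP_GameMode check it before the actor is destroyed after a delay.
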(event `self.ReceiveAnyDamage`
  (params (Damage :type "Float (single-precision)") (DamageType :type "DamageType Object Reference") (InstigatedBy :type "Controller Object Reference") (DamageCauser :type "Actor Object Reference"))
  (bind _mesh (`self.Mesh`))
  (bind _capsulecomponent (`self.CapsuleComponent`))
  (bind _humanhudref (`self.HumanHudRef`))
  ; Human Death Event
  (`/Engine/EditorBlueprintResources/StandardMacros.DoOnce` false
    (:`Completed`
      (`PrimitiveComponent.SetCollisionProfileName` _mesh "Ragdoll" true)
      (`PrimitiveComponent.SetCollisionResponseToChannel` _mesh "ECC_Pawn" "ECR_Ignore")
      (`PrimitiveComponent.SetSimulatePhysics` _mesh true)
      (`PrimitiveComponent.SetCollisionResponseToChannel` _capsulecomponent "ECC_Pawn" "ECR_Ignore")
      (`PrimitiveComponent.SetCollisionResponseToChannel` _capsulecomponent "ECC_Camera" "ECR_Ignore")
      (`PrimitiveComponent.SetPhysicsLinearVelocity` (`self.Mesh`) (* (`KismetMathLibrary.GetForwardVector` (`self.GetControlRotation`)) -9000.0) true "None")
      (`GameplayStatics.PlaySoundAtLocation` "/Game/SFX/Humangrunts/SC_Humanpain.SC_Humanpain" (`self.K2_GetActorLocation`) (struct) 1.0 1.0 0.0 null null null null)
      (`NiagaraFunctionLibrary.SpawnSystemAttached` "/Game/VFX/NS_Blood.NS_Blood" (`self.Mesh`) "None" (0.0 0.0 0.0) (struct) "KeepRelativeOffset")
      (bind _result (`/Engine/EditorBlueprintResources/StandardMacros.DecrementInt` (`/Game/Widgets/WB_Humans.humans` _humanhudref))
        (:`  `
          (set `/Game/Widgets/WB_Humans.humans` _result _humanhudref)
          (`/Game/Widgets/WB_Humans.update humans` (`self.HumanHudRef`))
          ;; Checks how many humans are dead
          (bind _asbp_game_mode (cast `/Game/Blueprints/BP_GameMode` (`GameplayStatics.GetGameMode`)))
          (`/Game/Blueprints/BP_GameMode.CheckHumanCount` _asbp_game_mode)
          (`KismetSystemLibrary.Delay` 2.0)
          (`self.K2_DestroyActor`))))))

(event `self.PawnSensing.OnSeePawn`
  (params (Pawn :type "Pawn Object Reference"))
  ; Chase Player When AI Spots Them
  (`|AIMoveTo` self (0.0 0.0 0.0) (`GameplayStatics.GetPlayerCharacter` 0) 15.0 :!label _label
    (:`OnSuccess`
      (`/Engine/EditorBlueprintResources/StandardMacros.DoOnce` false :!label _label_2
        (:`Completed`
          (`|PlayMontage` (`self.Mesh`) "/Game/Man/Demo/Animations/A_Manpunch_Montage.A_Manpunch_Montage"
            (:`OnCompleted`
              (goto _label_2 :!via `Reset`))
            (:`OnInterrupted`
              (goto _label_2 :!via `Reset`))))))))

(event `self.ReceiveBeginPlay`
  ; Chase Player When AI Spots Them
  (`PrimitiveComponent.SetCollisionEnabled` (`self.Sphere`) "NoCollision")
  (goto _label))

(event `Toggle Human Collision`
  (params (`true?` :type Boolean))
  (bind _sphere (`self.Sphere`))
  ; Toggle hand Collision
  (if `true?`
    (`PrimitiveComponent.SetCollisionEnabled` _sphere "QueryAndPhysics")
    (else
      (`PrimitiveComponent.SetCollisionEnabled` _sphere "NoCollision"))))

(event `self.Sphere.OnComponentBeginOverlap`
  (params (OverlappedComponent :type "PrimitiveComponent Object Reference") (OtherActor :type "Actor Object Reference") (OtherComp :type "PrimitiveComponent Object Reference") (OtherBodyIndex :type Integer) (bFromSweep :type Boolean) (SweepResult :type "HitResult Structure (by ref)"))
  (bind _returnvalue (`GameplayStatics.GetPlayerCharacter` 0))
  ; Apply Damage To Player
  (if (== OtherActor _returnvalue)
    (`GameplayStatics.ApplyDamage` _returnvalue 1.0)))

(fn `UserConstructionScript`)